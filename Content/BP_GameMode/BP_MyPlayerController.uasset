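; Player controller that sets up Enhanced Input and moves the player character.
; On BeginPlay it adds the default mapping context to the local player's input subsystem.
; The move action feeds its X and Y values into character movement along fixed world X and Y axes, independent of control rotation.
; An unconnected float-compare branch that would reset control rotation never runs.
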(event `self.ReceiveBeginPlay`
  (message `EnhancedInputSubsystemInterface.AddMappingContext` (pcsubsystem `EnhancedInputLocalPlayerSubsystem` (`GameplayStatics.GetPlayerController` 0)) "/Game/InputAction/IMC_Default.IMC_Default" 0 (struct)))

(event `EnhancedInput|/Game/InputAction/IA_Move`
  (params (ActionValue :type "Vector2D Structure") (ElapsedSeconds :type "Float (double-precision)") (TriggeredSeconds :type "Float (double-precision)") (InputAction :type "InputAction Object Reference" :default "/Game/InputAction/IA_Move.IA_Move"))
  (bind _returnvalue (`GameplayStatics.GetPlayerCharacter` 0))
  (:`Triggered`
    (`Pawn.AddMovementInput` _returnvalue (1.0 0.0 0.0) ActionValue_X false)
    (`Pawn.AddMovementInput` _returnvalue (0.0 1.0 0.0) ActionValue_Y false)))

(fn `UserConstructionScript`)