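; BP_MyGameModeBase is a game mode that runs the startup screen sequence on BeginPlay.
; It shows an opening background widget, waits briefly, then displays the SGA logo widget for a short time.
; It then removes the logo and adds the game title, melee idle and main menu widgets over the background, which stays on screen.
; Timing is handled with fixed Delay nodes, and all widgets are owned by the first player controller.
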(event `self.ReceiveBeginPlay`
  (bind _returnvalue (`GameplayStatics.GetPlayerController` 0))
  (bind _returnvalue_2 (`|CreateWidget` "/Game/BP_Widget/WBP_Widget_OpeningBackGround.WBP_Widget_OpeningBackGround_C" (`GameplayStatics.GetPlayerController` 0)))
  (`UserWidget.AddToViewport` _returnvalue_2 0)
  (`KismetSystemLibrary.Delay` 2.0)
  (bind _returnvalue_3 (`|CreateWidget` "/Game/BP_Widget/WBP_Widget_SGALOGO.WBP_Widget_SGALOGO_C" (`GameplayStatics.GetPlayerController` 0)))
  (`UserWidget.AddToViewport` _returnvalue_3 0)
  (`KismetSystemLibrary.Delay` 2.0)
  (`Widget.RemoveFromParent` _returnvalue_3)
  (bind _returnvalue_4 (`|CreateWidget` "/Game/BP_Widget/WBP_Widget_MainMenu.WBP_Widget_MainMenu_C" _returnvalue))
  (bind _returnvalue_5 (`|CreateWidget` "/Game/BP_Widget/WBP_Widget_Melee_Idle.WBP_Widget_Melee_Idle_C" _returnvalue))
  (bind _returnvalue_6 (`|CreateWidget` "/Game/BP_Widget/WBP_Widget_GameTitleOnMain.WBP_Widget_GameTitleOnMain_C" _returnvalue))
  (`UserWidget.AddToViewport` _returnvalue_6 0)
  (`UserWidget.AddToViewport` _returnvalue_5 0)
  (`UserWidget.AddToViewport` _returnvalue_4 0))

(fn `UserConstructionScript`)